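; BP_Traps is a placed trap shell that becomes a specific trap type and can be sold back for player gold.
; Initiate uses a selection index to set the mesh, child trap actor class and collision/cube width, then caches the player character.
; Enemies entering the collision send an activation message to the child trap actor.
; Sell-target state drives a DoOnce-gated yellow highlight material, and Sell credits gold before destroying the actor.
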(event `Sell`
  (bind _as_bp_third_person_character (`self.As BP Third Person Character`))
  (set `/Game/ThirdPerson/Blueprints/BP_ThirdPersonCharacter.Gold` (+ (`/Game/ThirdPerson/Blueprints/BP_ThirdPersonCharacter.Gold` _as_bp_third_person_character) (`self.Sell_Value`)) _as_bp_third_person_character)
  (`self.K2_DestroyActor`))

(event `Is_Sell_Target`
  (params (NewParam :type Boolean))
  (bind _trapmesh (`self.TrapMesh`))
  (set `self.Sell_Target` NewParam)
  (if (`self.Sell_Target`)
    (`/Engine/EditorBlueprintResources/StandardMacros.DoOnce` false :!label _label
      (:`Completed`
        (`PrimitiveComponent.SetMaterial` _trapmesh 0 "/Game/Environment/Traps/TrapsPreviewYellow.TrapsPreviewYellow")
        (goto _label_2 :!via `Reset`)))
    (else
      (`/Engine/EditorBlueprintResources/StandardMacros.DoOnce` false :!label _label_2
        (:`Completed`
          (`PrimitiveComponent.SetMaterial` _trapmesh 0 "/Game/Environment/Traps/TrapsMaterial.TrapsMaterial")
          (goto _label :!via `Reset`))))))

(event `self.TrapCollision.OnComponentBeginOverlap`
  (params (OverlappedComponent :type "PrimitiveComponent Object Reference") (OtherActor :type "Actor Object Reference") (OtherComp :type "PrimitiveComponent Object Reference") (OtherBodyIndex :type Integer) (bFromSweep :type Boolean) (SweepResult :type "HitResult Structure (by ref)"))
  (if (`self.ActorHasTag` OtherActor "enemy")
    (message `/Game/Blueprints/BPI_TrapActivasion.Trap_Activasion` (`|GetArrayItem` (`self.GetAllChildActors` true)))))

(event `Initiate`
  (params (TrapSelectionIndex :type Integer))
  (bind _cube (`self.Cube`))
  (bind _trapcollision (`self.TrapCollision`))
  (bind (_returnvalue_x _returnvalue_y _returnvalue_z) (`KismetMathLibrary.BreakVector` (`SceneComponent.K2_GetComponentScale` _cube)))
  (bind (_returnvalue_x_2 _returnvalue_y_2 _returnvalue_z_2) (`KismetMathLibrary.BreakVector` (`SceneComponent.K2_GetComponentScale` _trapcollision)))
  (bind _output_get (set `self.Trap Selection Index` TrapSelectionIndex))
  (`|ExecutionSequence`
    (:`then_0`
      (`StaticMeshComponent.SetStaticMesh` (`self.TrapMesh`) (select `int` _output_get :`0` "/Game/Environment/Traps/Trap_Fire.Trap_Fire" :`1` "/Game/Environment/Traps/Trap_Fire.Trap_Fire" :`2` "/Game/Environment/Traps/Trap_SawBladeFloor.Trap_SawBladeFloor" :!type "StaticMesh Object Reference"))
      (`ChildActorComponent.SetChildActorClass` (`self.Trap_Actor`) (select `int` _output_get :`0` "/Game/Blueprints/traps/BP_Cutter_Trap.BP_Cutter_Trap_C" :`1` "/Game/Blueprints/traps/BP_Hammer_Trap.BP_Hammer_Trap_C" :`2` null :!type "Actor Class Reference"))
      (`SceneComponent.SetWorldScale3D` _trapcollision (`KismetMathLibrary.MakeVector` _returnvalue_x_2 (* _returnvalue_y_2 (select `int` _output_get :`0` 1.0 :`1` 1.0 :`2` 2.0)) _returnvalue_z_2))
      (`SceneComponent.SetWorldScale3D` _cube (`KismetMathLibrary.MakeVector` _returnvalue_x (* _returnvalue_y (select `int` _output_get :`0` 1.0 :`1` 1.0 :`2` 2.0)) _returnvalue_z)))
    (:`then_1`
      (bind _asbp_third_person_character (cast `/Game/ThirdPerson/Blueprints/BP_ThirdPersonCharacter` (`GameplayStatics.GetPlayerCharacter` 0)))
      (set `self.As BP Third Person Character` _asbp_third_person_character))))

(fn `UserConstructionScript`)