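; BP_GameManager runs enemy waves and tracks a trap level that it broadcasts through a dispatcher.
; When ready, a wave start raises difficulty, scales the enemy count, updates the player UI and starts a looping spawn timer.
; Randomly scaled enemies spawn at one of two points by wave parity until the count pauses the timer.
; Removing the last tracked enemy re-arms the next wave after a short delay.
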(event `Trap_Level_Update`
  (bind _result (`/Engine/EditorBlueprintResources/StandardMacros.IncrementInt` (`self.Trap_Level`))
    (:`  `
      (`self.Trap_Level_Dispatcher` _result))))

(event `self.ReceiveBeginPlay`
  (bind _asbp_third_person_character (cast `/Game/ThirdPerson/Blueprints/BP_ThirdPersonCharacter` (`GameplayStatics.GetPlayerCharacter` 0)))
  (set `self.As BP Third Person Character` _asbp_third_person_character)
  (bind _returnvalue (`GameplayStatics.GetActorOfClass` "/Game/Blueprints/BP_LevelEnd.BP_LevelEnd_C"))
  (set `self.Level_End` _returnvalue)
  (`KismetSystemLibrary.DelayUntilNextTick`)
  (`self.Trap_Level_Update`))

(event `Initiate_wave`
  (if (`self.Next_Wave_Ready`)
    (set `self.Next_Wave_Ready` false)
    (`/Engine/EditorBlueprintResources/StandardMacros.IncrementInt` (`self.Wave Count`)
      (:`  `
        (bind _result (`/Engine/EditorBlueprintResources/StandardMacros.IncrementInt` (`self.Difficulty`))
          (:`  `
            (set `self.EnemCountPerWave` (* _result 10))
            (`/Game/Blueprints/WBP_User_Interface.Wave_Update` (`/Game/ThirdPerson/Blueprints/BP_ThirdPersonCharacter.WBP_UI_Ref` (`self.As BP Third Person Character`)) (`self.Wave Count`))
            (bind _returnvalue (`KismetSystemLibrary.K2_SetTimerDelegate` (delegate `Spawn_Enemy`) 1.0 true))
            (set `self.Timer_Handle` _returnvalue)))))))

(event `Spawn_Enemy`
  (bind _returnvalue (`|SpawnActorFromClass` "/Game/Blueprints/BP_Enemy_Test.BP_Enemy_Test_C" (`KismetMathLibrary.MakeTransform` (`|GetArrayItem` (`self.SpawnPoint`) (mod (`self.Wave Count`) 2)) (struct) (`KismetMathLibrary.Conv_DoubleToVector` (`KismetMathLibrary.RandomFloatInRange` 0.8 1.2))) "AlwaysSpawn" "MultiplyWithRoot" null null))
  (`KismetArrayLibrary.Array_Add` (`self.Enemies_on_stage`) _returnvalue)
  (bind _result (`/Engine/EditorBlueprintResources/StandardMacros.IncrementInt` (`self.Enemy_spawned`))
    (:`  `
      (if (>= _result (`self.EnemCountPerWave`))
        (`KismetSystemLibrary.K2_PauseTimerHandle` (`self.Timer_Handle`))
        (set `self.Enemy_spawned` 0)))))

(event `Wave_update`
  (params (NewParam :type "/Game/Blueprints/BP_Enemy_Test Object Reference"))
  (bind _enemies_on_stage (`self.Enemies_on_stage`))
  (`KismetArrayLibrary.Array_RemoveItem` _enemies_on_stage NewParam)
  (if (<= (`KismetArrayLibrary.Array_Length` _enemies_on_stage) 0)
    (`KismetSystemLibrary.Delay` 3.0)
    (set `self.Next_Wave_Ready` true)))

(fn `UserConstructionScript`)