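; Cutter trap that raises a spinning blade to damage tagged enemies inside its hitbox.
; Activation runs timelines for rise, wind-up, wind-down and fall, with a fast looping timer spinning the blade for the set duration between them.
; Overlap events maintain the enemy list that the spin loop damages, and a DoOnce gate blocks reactivation until the cooldown ends.
; The game manager's trap-level dispatcher increases damage and duration.
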(event `Trap_Level_Update`
  (params (`Trap Level` :type Integer))
  (set `self.Damage` (+ (* `Trap Level` 0.25) (`self.Damage`)))
  (set `self.Duration` (+ (`self.Duration`) (* (`KismetMathLibrary.Conv_IntToDouble` `Trap Level`) 0.25))))

(event `self.ReceiveBeginPlay`
  (bind _returnvalue (`GameplayStatics.GetActorOfClass` "/Game/Blueprints/BP_GameManager.BP_GameManager_C"))
  (add `/Game/Blueprints/BP_GameManager.Trap_Level_Dispatcher` _returnvalue (delegate `Trap_Level_Update`)))

(event `/Game/Blueprints/BPI_TrapActivasion.Trap_Activasion`
  (bind _trap_cutter (`self.Trap_Cutter`))
  (bind _trap_cutter_2 (`self.Trap_Cutter`))
  (bind _trap_cutter_3 (`self.Trap_Cutter`))
  (bind (_relativerotation_roll _relativerotation_pitch _relativerotation_yaw) (`KismetMathLibrary.BreakRotator` (`SceneComponent.RelativeRotation` _trap_cutter_3)))
  (bind (_relativerotation_roll_2 _relativerotation_pitch_2 _relativerotation_yaw_2) (`KismetMathLibrary.BreakRotator` (`SceneComponent.RelativeRotation` _trap_cutter_2)))
  (`/Engine/EditorBlueprintResources/StandardMacros.DoOnce` false :!label _label
    (:`Completed`
      ;[1 0.01138 0 0.5] Rise
      (bind (_direction _newtrack_0) (`Timeline|Rise` :!via `PlayFromStart`)
        (:`Update`
          (`SceneComponent.K2_SetRelativeLocation` (`self.Trap_Cutter`) (`KismetMathLibrary.VLerp` (0.0 0.0 -200.0) (0.0 0.0 0.0) _newtrack_0) false false))
        (:`Finished`
          ;[1 0.3111 0 0.5] Wind-up
          (set `self.Trap_active` true)
          (bind (_direction_2 _newtrack_0_2) (`Timeline|Wind_up` :!via `PlayFromStart`)
            (:`Update`
              (`SceneComponent.K2_SetRelativeRotation` _trap_cutter_3 (`KismetMathLibrary.MakeRotator` _relativerotation_roll _relativerotation_pitch (+ _relativerotation_yaw (* _newtrack_0_2 15.0))) false false)
              ;[1 0.8653 0 0.5] Spin
              (message `/Game/Blueprints/BPI_Damage.Damaged` (stale `Spin` _array_element) (`self.Damage`) (`self.Delay`) :!label _label_2))
            (:`Finished`
              (bind _returnvalue (`KismetSystemLibrary.K2_SetTimerDelegate` (delegate `Spin`) 0.001 true true))
              (`KismetSystemLibrary.Delay` (`self.Duration`))
              (`KismetSystemLibrary.K2_ClearAndInvalidateTimerHandle` _returnvalue)
              ;[0.7047 1 0 0.5] Wind_down
              (bind (_direction_3 _newtrack_0_3) (`Timeline|Wind_down` :!via `PlayFromStart`)
                (:`Update`
                  (`SceneComponent.K2_SetRelativeRotation` _trap_cutter_2 (`KismetMathLibrary.MakeRotator` _relativerotation_roll_2 _relativerotation_pitch_2 (+ _relativerotation_yaw_2 (* _newtrack_0_3 15.0))) false false))
                (:`Finished`
                  ;[0.1033 1 0 0.5] Stop
                  (set `self.Trap_active` false)
                  (`|ExecutionSequence`
                    (:`then_0`
                      (bind (_direction_4 _fall) (`Timeline|Fall` :!via `PlayFromStart`)
                        (:`Update`
                          (`SceneComponent.K2_SetRelativeLocation` (`self.Trap_Cutter`) (`KismetMathLibrary.VLerp` (0.0 0.0 -200.0) (0.0 0.0 0.0) _fall) false false))
                        (:`Finished`
                          (`self.Cooldown_Reset`))))
                    (:`then_1`
                      (`KismetSystemLibrary.Delay` 0.2)
                      (bind (_direction_5 _newtrack_0_4) (`Timeline|Timeline` :!via `PlayFromStart`)
                        (:`Update`
                          (`SceneComponent.K2_SetRelativeRotation` _trap_cutter (`KismetMathLibrary.RLerp` (`SceneComponent.RelativeRotation` _trap_cutter) (struct) _newtrack_0_4 true) false false))))))))))))))

(event `Cooldown_Reset`
  (`KismetSystemLibrary.Delay` (`self.Cooldown`))
  (goto _label :!via `Reset`))

(event `Spin`
  (bind _trap_cutter (`self.Trap_Cutter`))
  (bind (_relativerotation_roll _relativerotation_pitch _relativerotation_yaw) (`KismetMathLibrary.BreakRotator` (`SceneComponent.RelativeRotation` _trap_cutter)))
  ;[1 0.8653 0 0.5] Spin
  (`SceneComponent.K2_SetRelativeRotation` _trap_cutter (`KismetMathLibrary.MakeRotator` _relativerotation_roll _relativerotation_pitch (+ _relativerotation_yaw 15.0)) false false)
  (for _array_element (`self.Enemies_in_range`)
    (goto _label_2)))

(event `self.Hitbox.OnComponentBeginOverlap`
  (params (OverlappedComponent :type "PrimitiveComponent Object Reference") (OtherActor :type "Actor Object Reference") (OtherComp :type "PrimitiveComponent Object Reference") (OtherBodyIndex :type Integer) (bFromSweep :type Boolean) (SweepResult :type "HitResult Structure (by ref)"))
  (if (`self.ActorHasTag` OtherActor "Enemy")
    (`KismetArrayLibrary.Array_AddUnique` (`self.Enemies_in_range`) OtherActor)))

(event `self.Hitbox.OnComponentEndOverlap`
  (params (OverlappedComponent :type "PrimitiveComponent Object Reference") (OtherActor :type "Actor Object Reference") (OtherComp :type "PrimitiveComponent Object Reference") (OtherBodyIndex :type Integer))
  (`KismetArrayLibrary.Array_RemoveItem` (`self.Enemies_in_range`) OtherActor))

(fn `UserConstructionScript`)