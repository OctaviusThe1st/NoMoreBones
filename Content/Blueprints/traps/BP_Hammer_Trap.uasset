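; Hammer trap that, once activated, rises, bows, swipes, unbows and lowers through chained timelines, then waits out a cooldown behind a DoOnce.
; A sphere overlap tracks Enemy-tagged actors in range.
; During the swipe, two delayed hits send damage and knockback messages to those targets, pushing them away from the trap with distance-independent strength.
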(event `/Game/Blueprints/BPI_TrapActivasion.Trap_Activasion`
  (`/Engine/EditorBlueprintResources/StandardMacros.DoOnce` false :!label _label
    (:`Completed`
      ;[0.05418 1 0 0.5] Animation
      (bind (_direction _newtrack_0) (`Timeline|Rise` :!via `PlayFromStart`)
        (:`Update`
          (`SceneComponent.K2_SetRelativeLocation` (`self.handle`) (`KismetMathLibrary.VLerp` (0.0 0.0 -400.0) (0.0 0.0 150.0) _newtrack_0) false false))
        (:`Finished`
          (bind (_direction_2 _newtrack_0_2) (`Timeline|Bow` :!via `PlayFromStart`)
            (:`Update`
              (`SceneComponent.K2_SetRelativeRotation` (`self.hammer`) (`KismetMathLibrary.RLerp` (struct :`Yaw` 180.0 :`Roll` 180.0) (struct :`Pitch` 100.0 :`Yaw` 180.0 :`Roll` 180.0) _newtrack_0_2) false false))
            (:`Finished`
              (`|ExecutionSequence`
                (:`then_0`
                  (bind (_direction_3 _newtrack_0_3) (`Timeline|Swipe` :!via `PlayFromStart`)
                    (:`Update`
                      (`SceneComponent.K2_SetRelativeRotation` (`self.hammer`) (`KismetMathLibrary.RLerp` (struct :`Pitch` 100.0 :`Yaw` 180.0 :`Roll` 180.0) (`KismetMathLibrary.MakeRotator` 180.0 100.0 (+ (* _newtrack_0_3 180.0) 180.0)) _newtrack_0_3) false false))
                    (:`Finished`
                      (bind (_direction_4 _newtrack_0_4) (`Timeline|Un-Bow` :!via `PlayFromStart`)
                        (:`Update`
                          (`SceneComponent.K2_SetRelativeRotation` (`self.hammer`) (`KismetMathLibrary.RLerp` (struct :`Yaw` 180.0 :`Roll` 180.0) (struct :`Pitch` 100.0 :`Yaw` 180.0 :`Roll` 180.0) _newtrack_0_4) false false))
                        (:`Finished`
                          (bind (_direction_5 _newtrack_0_5) (`Timeline|Fall` :!via `PlayFromStart`)
                            (:`Update`
                              (`SceneComponent.K2_SetRelativeLocation` (`self.handle`) (`KismetMathLibrary.VLerp` (0.0 0.0 -500.0) (0.0 0.0 150.0) _newtrack_0_5) false false))
                            (:`Finished`
                              (`self.Cooldown_Reset`))))))))
                (:`then_1`
                  (`KismetSystemLibrary.Delay` 0.3)
                  (`self.Hit`)
                  (`KismetSystemLibrary.Delay` 0.4)
                  (`self.Hit`))))))))))

(event `Cooldown_Reset`
  (`KismetSystemLibrary.Delay` (`self.Cooldown`))
  (goto _label :!via `Reset`))

(event `Hit`
  (for _array_element (`self.Targets_in_range`)
    (if (`self.ActorHasTag` _array_element "Enemy")
      (message `/Game/Blueprints/BPI_Damage.Damaged` _array_element (`self.Damage`) (`self.Delay`))
      (bind _returnvalue (- (`self.K2_GetActorLocation` _array_element) (`self.K2_GetActorLocation`)))
      (message `/Game/Blueprints/BPI_Damage.Knockback` _array_element (* _returnvalue (`self.Knockback`) (* (/ 1.0 (`KismetMathLibrary.VSize` _returnvalue)) 500.0))))))

(event `self.Sphere.OnComponentBeginOverlap`
  (params (OverlappedComponent :type "PrimitiveComponent Object Reference") (OtherActor :type "Actor Object Reference") (OtherComp :type "PrimitiveComponent Object Reference") (OtherBodyIndex :type Integer) (bFromSweep :type Boolean) (SweepResult :type "HitResult Structure (by ref)"))
  (if (`self.ActorHasTag` OtherActor "Enemy")
    (`KismetArrayLibrary.Array_AddUnique` (`self.Targets_in_range`) OtherActor)))

(event `self.Sphere.OnComponentEndOverlap`
  (params (OverlappedComponent :type "PrimitiveComponent Object Reference") (OtherActor :type "Actor Object Reference") (OtherComp :type "PrimitiveComponent Object Reference") (OtherBodyIndex :type Integer))
  (`KismetArrayLibrary.Array_RemoveItem` (`self.Targets_in_range`) OtherActor))

(fn `UserConstructionScript`)