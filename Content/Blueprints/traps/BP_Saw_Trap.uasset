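; Saw trap that rises on activation, spins and travels along an InterpToMovement path while damaging enemies in range, then retracts and cools down.
; FlipFlop-driven timelines play forward and reverse to raise, speed up, slow down and lower the saw.
; A fast looping timer rotates the blade and damages tagged enemies tracked by box overlaps.
; BP_GameManager's trap-level dispatcher increases damage and shortens cooldown.
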(event `Trap_Level_Update`
  (params (`Trap Level` :type Integer))
  (set `self.Damage` (+ (* `Trap Level` 0.005) (`self.Damage`)))
  (set `self.Cooldown` (- (`self.Cooldown`) (/ (`KismetMathLibrary.Conv_IntToDouble` `Trap Level`) 10.0))))

(event `self.ReceiveBeginPlay`
  (`KismetSystemLibrary.DelayUntilNextTick`)
  (`SceneComponent.K2_SetRelativeLocation` (`self.DefaultSceneRoot`) (0.0 200.0 0.0) false false)
  (bind _returnvalue (`GameplayStatics.GetActorOfClass` "/Game/Blueprints/BP_GameManager.BP_GameManager_C"))
  (add `/Game/Blueprints/BP_GameManager.Trap_Level_Dispatcher` _returnvalue (delegate `Trap_Level_Update`)))

(event `/Game/Blueprints/BPI_TrapActivasion.Trap_Activasion`
  (bind _interptomovement (`self.InterpToMovement`))
  (bind _interptomovement_2 (`self.InterpToMovement`))
  (`/Engine/EditorBlueprintResources/StandardMacros.DoOnce` false :!label _label
    (:`Completed`
      (bind _isa (`/Engine/EditorBlueprintResources/StandardMacros.FlipFlop` :!label _label_2)
        (:`A`
          (bind (_direction _newtrack_0) (`Timeline|Timeline` :!via `PlayFromStart` :!label _label_3)
            (:`Update`
              (`SceneComponent.K2_SetRelativeLocation` (`self.Cube`) (`KismetMathLibrary.VLerp` (0.0 0.0 -150.0) (0.0 0.0 10.0) _newtrack_0) false true))
            (:`Finished`
              (if _isa
                (bind _returnvalue (`KismetSystemLibrary.K2_SetTimerDelegate` (delegate `Spin`) 0.001 true true))
                (`ActorComponent.SetActive` _interptomovement_2 true true)
                (`InterpToMovementComponent.RestartMovement` _interptomovement_2 1.0)
                (bind _isa_2 (`/Engine/EditorBlueprintResources/StandardMacros.FlipFlop` :!label _label_4)
                  (:`A`
                    (bind (_direction_2 _newtrack_0_2) (`Timeline|Timeline_1` :!via `PlayFromStart` :!label _label_5)
                      (:`Update`
                        (set `InterpToMovementComponent.SpeedMultiplier` (* (+ _newtrack_0_2 1.0) 1.0) _interptomovement))
                      (:`Finished`
                        (if _isa_2
                          (goto _label_4)
                          (else
                            (`KismetSystemLibrary.K2_ClearAndInvalidateTimerHandle` _returnvalue)
                            (`ActorComponent.SetActive` _interptomovement false true)
                            (goto _label_2))))))
                  (:`B`
                    (goto _label_5 :!via `ReverseFromEnd`)))
                (else
                  (`SceneComponent.K2_SetRelativeLocation` (`self.DefaultSceneRoot`) (0.0 200.0 0.0) false false)
                  (`KismetSystemLibrary.Delay` (`self.Cooldown`))
                  (goto _label :!via `Reset`))))))
        (:`B`
          (goto _label_3 :!via `ReverseFromEnd`))))))

(event `Spin`
  (bind _trap_sawblade (`self.Trap_SawBlade`))
  (bind _relativerotation_roll (`KismetMathLibrary.BreakRotator` (`SceneComponent.RelativeRotation` _trap_sawblade)))
  (`SceneComponent.K2_SetRelativeRotation` _trap_sawblade (`KismetMathLibrary.MakeRotator` (+ _relativerotation_roll (* (stale `/Game/Blueprints/BPI_TrapActivasion.Trap_Activasion` _newtrack_0_2) 15.0))) false false)
  (for _array_element (`self.Targets_in_range`)
    (message `/Game/Blueprints/BPI_Damage.Damaged` _array_element (`self.damage`) (`self.delay`))))

(event `self.Box.OnComponentBeginOverlap`
  (params (OverlappedComponent :type "PrimitiveComponent Object Reference") (OtherActor :type "Actor Object Reference") (OtherComp :type "PrimitiveComponent Object Reference") (OtherBodyIndex :type Integer) (bFromSweep :type Boolean) (SweepResult :type "HitResult Structure (by ref)"))
  (if (`self.ActorHasTag` OtherActor "Enemy")
    (`KismetArrayLibrary.Array_AddUnique` (`self.Targets_in_range`) OtherActor)))

(event `self.Box.OnComponentEndOverlap`
  (params (OverlappedComponent :type "PrimitiveComponent Object Reference") (OtherActor :type "Actor Object Reference") (OtherComp :type "PrimitiveComponent Object Reference") (OtherBodyIndex :type Integer))
  (`KismetArrayLibrary.Array_RemoveItem` (`self.Targets_in_range`) OtherActor))

(fn `UserConstructionScript`)