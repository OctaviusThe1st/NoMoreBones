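; Saw blade trap that, when activated, damages Enemy-tagged actors inside its box trigger.
; TrapActivasion, gated by a DoOnce, moves the cube by timeline and restarts InterpTo movement, then starts a looping Spin timer that is never cleared.
; Spin rolls the blade at a timeline-scaled rate and sends damage messages to overlapping targets.
; Later, movement stops and another timeline moves the cube, triggering the cooldown that re-arms the DoOnce.
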(event `self.ReceiveBeginPlay`)

(event `/Game/Blueprints/BPI_TrapActivasion.Trap_Activasion`
  (`/Engine/EditorBlueprintResources/StandardMacros.DoOnce` false :!label _label
    (:`Completed`
      (bind (_direction _newtrack_0) (`Timeline|Timeline` :!via `PlayFromStart`)
        (:`Update`
          (`SceneComponent.K2_SetRelativeLocation` (`self.Cube`) (`KismetMathLibrary.VLerp` (0.0 0.0 -150.0) (0.0 0.0 0.0) _newtrack_0) false false)
          (`InterpToMovementComponent.RestartMovement` (`self.InterpToMovement`) 1.0))
        (:`Finished`
          (`KismetSystemLibrary.K2_SetTimerDelegate` (delegate `Spin`) 0.001 true true)
          (bind (_direction_2 _newtrack_0_2) (`Timeline|Timeline_1` :!via `PlayFromStart`)
            (:`Finished`
              (`KismetSystemLibrary.Delay` 3.0)
              (`MovementComponent.StopMovementImmediately` (`self.InterpToMovement`))
              (bind (_direction_3 _newtrack_0_3) (`Timeline|Timeline_2` :!via `PlayFromStart`)
                (:`Update`
                  (`SceneComponent.K2_SetRelativeLocation` (`self.Cube`) (`KismetMathLibrary.VLerp` (0.0 0.0 -150.0) (0.0 0.0 0.0) _newtrack_0_3) false false)
                  (`self.Reset`))))))))))

(event `Reset`
  (`KismetSystemLibrary.Delay` (`self.Cooldown`))
  (goto _label :!via `Reset`))

(event `Spin`
  (bind _trap_sawblade (`self.Trap_SawBlade`))
  (bind _relativerotation_roll (`KismetMathLibrary.BreakRotator` (`SceneComponent.RelativeRotation` _trap_sawblade)))
  (`SceneComponent.K2_SetRelativeRotation` _trap_sawblade (`KismetMathLibrary.MakeRotator` (+ _relativerotation_roll (* (stale `/Game/Blueprints/BPI_TrapActivasion.Trap_Activasion` _newtrack_0_2) 20.0))) false false)
  (for _array_element (`self.Targets_in_range`)
    (message `/Game/Blueprints/BPI_Damage.Damaged` _array_element (`self.damage`) (`self.delay`))))

(event `self.Box.OnComponentBeginOverlap`
  (params (OverlappedComponent :type "PrimitiveComponent Object Reference") (OtherActor :type "Actor Object Reference") (OtherComp :type "PrimitiveComponent Object Reference") (OtherBodyIndex :type Integer) (bFromSweep :type Boolean) (SweepResult :type "HitResult Structure (by ref)"))
  (if (`self.ActorHasTag` OtherActor "Enemy")
    (`KismetArrayLibrary.Array_AddUnique` (`self.Targets_in_range`) OtherActor)))

(event `self.Box.OnComponentEndOverlap`
  (params (OverlappedComponent :type "PrimitiveComponent Object Reference") (OtherActor :type "Actor Object Reference") (OtherComp :type "PrimitiveComponent Object Reference") (OtherBodyIndex :type Integer))
  (`KismetArrayLibrary.Array_RemoveItem` (`self.Targets_in_range`) OtherActor))

(fn `UserConstructionScript`)