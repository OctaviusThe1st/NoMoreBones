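; BP_Arrow is a short-lived arrow projectile in the traps folder that destroys itself half a second after spawning.
; When its sphere overlaps a component tagged ArrowHit, it stops, attaches to that component, sends DamagedMessage to the owning actor and destroys itself after a brief delay.
; A blocking hit on an actor with the same tag only stops its movement.
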(event `self.ReceiveBeginPlay`
  (`KismetSystemLibrary.Delay` 0.5)
  (`self.K2_DestroyActor`))

(event `self.Sphere.OnComponentBeginOverlap`
  (params (OverlappedComponent :type "PrimitiveComponent Object Reference") (OtherActor :type "Actor Object Reference") (OtherComp :type "PrimitiveComponent Object Reference") (OtherBodyIndex :type Integer) (bFromSweep :type Boolean) (SweepResult :type "HitResult Structure (by ref)"))
  (if (`ActorComponent.ComponentHasTag` OtherComp "ArrowHit")
    (`MovementComponent.StopMovementImmediately` (`self.ProjectileMovement`))
    (`self.K2_AttachToComponent` OtherComp "None" "KeepWorld" "KeepWorld" "KeepWorld")
    (message `/Game/Blueprints/BPI_Damage.Damaged` OtherActor 10.0 0.1)
    (`KismetSystemLibrary.Delay` 0.2)
    (`self.K2_DestroyActor`)))

(event `self.ReceiveHit`
  (params (MyComp :type "PrimitiveComponent Object Reference") (Other :type "Actor Object Reference") (OtherComp :type "PrimitiveComponent Object Reference") (bSelfMoved :type Boolean) (HitLocation :type "Vector Structure") (HitNormal :type "Vector Structure") (NormalImpulse :type "Vector Structure") (Hit :type "HitResult Structure (by ref)"))
  (if (`self.ActorHasTag` Other "ArrowHit")
    (`MovementComponent.StopMovementImmediately` (`self.ProjectileMovement`))))

(fn `UserConstructionScript`)