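; Ballista trap turret that deploys on BeginPlay and shoots arrows at enemies within range.
; Chained timelines and FlipFlops raise the housing, open the doors, lift the turret, then close up again.
; Range overlaps maintain a list of Enemy-tagged actors, whose first entry becomes the target and unpauses a looping fire timer.
; Each shot turns the turret and spawns BP_Arrow, with magazine reloads and GameManager trap-level events adjusting magazine size and fire rate.
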(event `Trap_Level_Update`
  (params (`Trap Level` :type Integer))
  (set `self.Mag_size` (+ (* `Trap Level` 5) 5))
  (set `self.FireRate` (- (`self.FireRate`) (* (`KismetMathLibrary.Conv_IntToDouble` `Trap Level`) 0.02))))

(event `Target_Update`
  (bind _targets_in_range (`self.Targets_in_range`))
  (bind _timer_handle (`self.Timer_Handle`))
  (bind _output (`|GetArrayItem` _targets_in_range))
  ;[1 0.02404 0] Target_Update
  (`/Engine/EditorBlueprintResources/StandardMacros.Gate` true :!label _label
    (:`Exit`
      (if (> (`KismetArrayLibrary.Array_Length` _targets_in_range) 0)
        (`/Engine/EditorBlueprintResources/StandardMacros.IsValid` _output
          (:`Is Valid`
            (set `self.Active_Target` _output)
            (set `self.Trap_Active` true)
            (`KismetSystemLibrary.K2_UnPauseTimerHandle` _timer_handle))
          (:`Is Not Valid`
            (`self.Target_Update`)))
        (else
          (set `self.Trap_Active` false)
          (`KismetSystemLibrary.K2_PauseTimerHandle` _timer_handle))))))

(event `self.ReceiveBeginPlay`
  ;[0.007111 1 0 0.5] Opening Sequence
  (`|ExecutionSequence`
    (:`then_0`
      (bind _isa (`/Engine/EditorBlueprintResources/StandardMacros.FlipFlop` :!label _label_2)
        (:`A`
          (bind (_direction _base_rise) (`Timeline|Timeline` :!label _label_3)
            (:`Update`
              (`SceneComponent.K2_SetRelativeLocation` (`self.box_small`) (`KismetMathLibrary.VLerp` (0.0 0.0 -100.0) (0.0 0.0 0.0) _base_rise) false false))
            (:`Finished`
              (if _isa
                (bind _isa_2 (`/Engine/EditorBlueprintResources/StandardMacros.FlipFlop` :!label _label_4)
                  (:`A`
                    (bind (_direction_2 _base_rise_2) (`Timeline|Timeline_0` :!label _label_5)
                      (:`Update`
                        (`SceneComponent.K2_SetRelativeRotation` (`self.Right_Door`) (`KismetMathLibrary.RLerp` (struct) (struct :`Roll` 145.0) _base_rise_2) false false)
                        (`SceneComponent.K2_SetRelativeRotation` (`self.left_door`) (`KismetMathLibrary.RLerp` (struct) (struct :`Roll` -145.0) _base_rise_2) false false))
                      (:`Finished`
                        (if _isa_2
                          (bind (_direction_3 _base_rise_3) (`Timeline|Timeline_1`)
                            (:`Update`
                              (`SceneComponent.K2_SetRelativeLocation` (`self.Turret_Base`) (`KismetMathLibrary.VLerp` (0.0 0.0 -130.0) (0.0 0.0 250.0) _base_rise_3) false false))
                            (:`Finished`
                              (goto _label_4)))
                          (else
                            (goto _label_2))))))
                  (:`B`
                    (goto _label_5 :!via `Reverse`)))
                (else
                  ;[1 0.02404 0] Target_Update
                  (`|ExecutionSequence`
                    (:`then_0`
                      (goto _label :!via `Open`))
                    (:`then_1`
                      (`KismetSystemLibrary.DelayUntilNextTick`)
                      (`self.Target_Update`))))))))
        (:`B`
          (goto _label_3 :!via `Reverse`))))
    (:`then_1`
      ;[1 0 0.9107 0.5] Fire Loop
      (set `self.Current_Ammo` (`self.Mag_size`))
      (bind _returnvalue (`KismetSystemLibrary.K2_SetTimerDelegate` (delegate `Pewpew`) (`self.FireRate`) true false 0.0 0.1))
      (bind _output_get (set `self.Timer_Handle` _returnvalue))
      (`KismetSystemLibrary.K2_PauseTimerHandle` _output_get))
    (:`then_2`
      (bind _returnvalue_2 (`GameplayStatics.GetActorOfClass` "/Game/Blueprints/BP_GameManager.BP_GameManager_C"))
      (add `/Game/Blueprints/BP_GameManager.Trap_Level_Dispatcher` _returnvalue_2 (delegate `Trap_Level_Update`)))))

(event `Reload`
  (bind _timer_handle (`self.Timer_Handle`))
  ;[1 0 0.8425 0.5] Reload
  (`/Engine/EditorBlueprintResources/StandardMacros.DoOnce` false :!label _label_6
    (:`Completed`
      (`KismetSystemLibrary.K2_PauseTimerHandle` _timer_handle)
      (`KismetSystemLibrary.Delay` (`self.Reload_Time`))
      (set `self.Current_Ammo` (`self.Mag_size`))
      (`KismetSystemLibrary.K2_UnPauseTimerHandle` _timer_handle)
      (`self.Target_Update`)
      (goto _label_6 :!via `Reset`))))

(event `self.range.OnComponentBeginOverlap`
  (params (OverlappedComponent :type "PrimitiveComponent Object Reference") (OtherActor :type "Actor Object Reference") (OtherComp :type "PrimitiveComponent Object Reference") (OtherBodyIndex :type Integer) (bFromSweep :type Boolean) (SweepResult :type "HitResult Structure (by ref)"))
  (if (`self.ActorHasTag` OtherActor "Enemy")
    (`KismetArrayLibrary.Array_AddUnique` (`self.Targets_in_range`) OtherActor)
    (`self.Target_Update` :!label _label_7)))

(event `Arrow_Launcher`
  (bind _active_target (`self.Active_Target`))
  (bind _turret_base (`self.Turret_Base`))
  ; Comment
  (`|ExecutionSequence`
    (:`then_0`
      (`KismetSystemLibrary.Delay` 0.2)
      (`|SpawnActorFromClass` "/Game/Blueprints/traps/BP_Arrow.BP_Arrow_C" (`SceneComponent.K2_GetComponentToWorld` (`self.Arrow`)) "AlwaysSpawn" "MultiplyWithRoot" null null))
    (:`then_1`
      (bind (_direction _newtrack_0) (`Timeline|Timeline_2` :!via `PlayFromStart`)
        (:`Update`
          (if (`KismetSystemLibrary.IsValid` _active_target)
            (`SceneComponent.K2_SetWorldRotation` _turret_base (`KismetMathLibrary.RLerp` (`SceneComponent.K2_GetComponentRotation` _turret_base) (`KismetMathLibrary.FindLookAtRotation` (`SceneComponent.K2_GetComponentLocation` _turret_base) (`self.K2_GetActorLocation` _active_target)) _newtrack_0 true) false false)))))))

(event `self.range.OnComponentEndOverlap`
  (params (OverlappedComponent :type "PrimitiveComponent Object Reference") (OtherActor :type "Actor Object Reference") (OtherComp :type "PrimitiveComponent Object Reference") (OtherBodyIndex :type Integer))
  (`KismetArrayLibrary.Array_RemoveItem` (`self.Targets_in_range`) OtherActor)
  (goto _label_7))

(event `Pewpew`
  (bind _current_ammo (`self.Current_Ammo`))
  (bind _returnvalue (<= _current_ammo 0))
  ;[1 0 0.9107 0.5] Fire Loop
  (if _returnvalue
    (`self.Reload` :!label _label_8)
    (else
      (`/Engine/EditorBlueprintResources/StandardMacros.DecrementInt` _current_ammo
        (:`  `
          (`self.Arrow_Launcher`)
          (if _returnvalue
            (`KismetSystemLibrary.K2_PauseTimerHandle` (`self.Timer_Handle`))
            (goto _label_8)))))))

(fn `UserConstructionScript`)