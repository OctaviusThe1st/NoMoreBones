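; BP_Level_Panel is an interactable panel that sells trap level upgrades for the player's gold.
; On BeginPlay it caches the third-person character and the BP_GameManager actor.
; When Interact receives enough gold, it deducts the cost from the character, raises the next cost in proportion to the manager's Difficulty, and increments its level.
; It then prints the level and calls TrapLevelUpdate on the game manager.
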(event `self.ReceiveBeginPlay`
  (bind _asbp_third_person_character (cast `/Game/ThirdPerson/Blueprints/BP_ThirdPersonCharacter` (`GameplayStatics.GetPlayerCharacter` 0)))
  (set `self.As BP Third Person Character` _asbp_third_person_character)
  (bind _returnvalue (`GameplayStatics.GetActorOfClass` "/Game/Blueprints/BP_GameManager.BP_GameManager_C"))
  (set `self.As Game Manager` _returnvalue))

(event `/Game/Blueprints/BPI_Damage.Interact`
  (params (Gold :type "Float (double-precision)"))
  (bind _as_bp_third_person_character (`self.As BP Third Person Character`))
  (if (>= Gold (`self.Upgrade_Cost`))
    (set `/Game/ThirdPerson/Blueprints/BP_ThirdPersonCharacter.Gold` (- (`/Game/ThirdPerson/Blueprints/BP_ThirdPersonCharacter.Gold` _as_bp_third_person_character) (`self.Upgrade_Cost`)) _as_bp_third_person_character)
    (set `self.Upgrade_Cost` (+ (`self.Upgrade_Cost`) (* (`/Game/Blueprints/BP_GameManager.Difficulty` (`self.As Game Manager`)) 500.0)))
    (bind _result (`/Engine/EditorBlueprintResources/StandardMacros.IncrementInt` (`self.Level`))
      (:`  `
        (`KismetSystemLibrary.PrintString` (`KismetStringLibrary.Concat_StrStr` "Trap Level: " (`KismetStringLibrary.Conv_IntToString` _result)))
        (`/Game/Blueprints/BP_GameManager.Trap_Level_Update` (`self.As Game Manager`))))))

(fn `UserConstructionScript`)