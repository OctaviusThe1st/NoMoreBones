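; AI controller for an enemy that starts the BT_Enemy behavior tree on possess and carries an AI perception component.
; Its walk event issues an AI MoveTo toward a stored third-person character reference and prints a debug string on success.
; The timer-driven chase setup and perception-based pause/unpause logic are disconnected, so walk is never triggered here and the perception update handler does nothing.
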(event `self.ReceivePossess`
  (params (PossessedPawn :type "Pawn Object Reference"))
  (`self.RunBehaviorTree` "/Game/Blueprints/BT_Enemy.BT_Enemy"))

(event `self.ReceiveBeginPlay`)

(event `walk`
  (`|AIMoveTo` null (0.0 0.0 0.0) (`self.As BP Third Person Character`)
    (:`OnSuccess`
      (`KismetSystemLibrary.PrintString` "Hello"))))

(event `self.AIPerception.OnTargetPerceptionUpdated`
  (params (Actor :type "Actor Object Reference") (Stimulus :type "AIStimulus Structure")))

(fn `UserConstructionScript`)