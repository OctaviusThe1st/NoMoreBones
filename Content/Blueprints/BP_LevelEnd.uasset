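; BP_LevelEnd is the defended base at the end of the enemy path, which tracks base health and lets waves be started.
; Enemies entering its Box are destroyed with no gold reward and deal difficulty-scaled damage, updating the player's UI and calling Defeat on BP_GameManager at zero health.
; Interact calls InitiateWave on the manager and hides the text renders on first use.
; BeginPlay waits a tick before caching the UI and manager references.
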(event `self.ReceiveBeginPlay`
  (bind _output_get (set `self.Base_Max_HP` 500.0))
  (set `self.Base_Current_HP` _output_get)
  (bind _asbp_third_person_character (cast `/Game/Blueprints/BP_ThirdPersonCharacter` (`GameplayStatics.GetPlayerCharacter` 0)))
  (bind _output_get_2 (set `self.As BP Third Person Character` _asbp_third_person_character))
  (`KismetSystemLibrary.DelayUntilNextTick`)
  (bind _output_get_3 (set `self.WBP UI Ref` (`/Game/Blueprints/BP_ThirdPersonCharacter.WBP_UI_Ref` _output_get_2)))
  (bind _returnvalue (`GameplayStatics.GetActorOfClass` "/Game/Blueprints/BP_GameManager.BP_GameManager_C"))
  (set `self.As BP_GameManager` _returnvalue)
  (`/Game/Blueprints/WBP_User_Interface.Base_Health_Update` _output_get_3 (`self.Base_Max_HP`) (`self.Base_Current_HP`)))

(event `self.Box.OnComponentBeginOverlap`
  (params (OverlappedComponent :type "PrimitiveComponent Object Reference") (OtherActor :type "Actor Object Reference") (OtherComp :type "PrimitiveComponent Object Reference") (OtherBodyIndex :type Integer) (bFromSweep :type Boolean) (SweepResult :type "HitResult Structure (by ref)"))
  (bind _asbp_enemy_test (cast `/Game/Blueprints/BP_Enemy_Test` OtherActor))
  (set `/Game/Blueprints/BP_Enemy_Test.Gold_Reward` 0.0 _asbp_enemy_test)
  (`/Game/Blueprints/BP_Enemy_Test.Destroyed` _asbp_enemy_test)
  (bind _output_get (set `self.Base_Current_HP` (- (`self.Base_Current_HP`) (+ (* (`/Game/Blueprints/BP_GameManager.Difficulty` (`self.As BP_GameManager`)) 3) 25))))
  (`/Game/Blueprints/WBP_User_Interface.Base_Health_Update` (`self.WBP UI Ref`) (`self.Base_Max_HP`) _output_get)
  (if (<= (`self.Base_Current_HP`) 0.0)
    (`/Game/Blueprints/BP_GameManager.Defeat` (`self.As BP_GameManager`))))

(event `/Game/Blueprints/BPI_Damage.Interact`
  (params (Gold :type "Float (double-precision)"))
  (`/Game/Blueprints/BP_GameManager.Initiate_wave` (`self.As BP_GameManager`))
  (`/Engine/EditorBlueprintResources/StandardMacros.DoOnce` false
    (:`Completed`
      (`SceneComponent.SetVisibility` (`self.TextRender`) false false)
      (`SceneComponent.SetVisibility` (`self.TextRender1`) false false)
      (`SceneComponent.SetVisibility` (`self.TextRender2`) false false)
      (`SceneComponent.SetVisibility` (`self.TextRender3`) false false)
      (`SceneComponent.SetVisibility` (`self.TextRender4`) false false)
      (`SceneComponent.SetVisibility` (`self.TextRender5`) false false))))

(fn `UserConstructionScript`)