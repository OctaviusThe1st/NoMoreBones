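; Trap placement preview actor, parented to the third-person character, that shows the selected trap and whether its spot is clear.
; Mesh Update swaps the base and hologram meshes per trap type, adjusting collision scale and hologram transform.
; A looping timer spins the Root component.
; Overlaps with "Collision"-tagged actors are tracked to set the character's placement and overlap flags and switch preview materials between green and red.
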(event `Mesh_Update`
  (params (NewParam2 :type "/Game/Blueprints/Enum_Trap_Selection Enum" :default "NewEnumerator0"))
  (bind _cube (`self.Cube`))
  ;[1 0 0.6354 0.5] Base Update
  (`StaticMeshComponent.SetStaticMesh` (`self.TrapPreviewMesh`) (select `/Game/Blueprints/Enum_Trap_Selection` NewParam2 :`NewEnumerator0` "/Game/Environment/Traps/Trap_CutterFloor.Trap_CutterFloor" :`NewEnumerator1` "/Game/Environment/Traps/Trap_CutterFloor.Trap_CutterFloor" :`NewEnumerator2` "/Game/Environment/Traps/Trap_SawBladeFloor.Trap_SawBladeFloor" :`NewEnumerator3` "/Game/Environment/Traps/Trap_Fire.Trap_Fire" :!type "StaticMesh Object Reference"))
  (`SceneComponent.SetRelativeScale3D` (`self.TrapPreviewCollision`) (`KismetMathLibrary.MakeVector` 5.25 (* (select `/Game/Blueprints/Enum_Trap_Selection` NewParam2 :`NewEnumerator0` 1.0 :`NewEnumerator1` 1.0 :`NewEnumerator2` 2.0 :`NewEnumerator3` 1.0) 5.25) 0.25))
  ;[1 0 0.5924 0.5] Hologram Update
  (`StaticMeshComponent.SetStaticMesh` _cube (select `/Game/Blueprints/Enum_Trap_Selection` NewParam2 :`NewEnumerator0` "/Game/Environment/Traps/Trap_Cutter.Trap_Cutter" :`NewEnumerator1` "/Game/Environment/Traps/Trap_Hammer.Trap_Hammer" :`NewEnumerator2` "/Game/Environment/Traps/Trap_SawBlade.Trap_SawBlade" :`NewEnumerator3` "/Game/Characters/Adventurers/Equipments/crossbow_1handed.crossbow_1handed" :!type "StaticMesh Object Reference"))
  (`SceneComponent.K2_SetRelativeTransform` _cube (`KismetMathLibrary.MakeTransform` (`KismetMathLibrary.MakeVector` 0.0 (select `/Game/Blueprints/Enum_Trap_Selection` NewParam2 :`NewEnumerator1` -59.0 :`NewEnumerator3` -40.0) (select `/Game/Blueprints/Enum_Trap_Selection` NewParam2 :`NewEnumerator0` 260.0 :`NewEnumerator1` 300.0 :`NewEnumerator2` 300.0 :`NewEnumerator3` 300.0)) (`KismetMathLibrary.MakeRotator` (select `/Game/Blueprints/Enum_Trap_Selection` NewParam2 :`NewEnumerator1` 90.0)) (select `/Game/Blueprints/Enum_Trap_Selection` NewParam2 :`NewEnumerator0` (0.5 0.5 0.5) :`NewEnumerator1` (0.5 0.5 0.5) :`NewEnumerator2` (0.5 0.5 0.5) :`NewEnumerator3` (2.0 2.0 2.0) :!type "Vector Structure")) false false))

(event `self.ReceiveBeginPlay`
  ;[1 0.587 0 0.5] BeginPlay Setup
  (bind _asbp_third_person_character (cast `/Game/Blueprints/BP_ThirdPersonCharacter` (`self.GetParentActor`)))
  (set `self.As BP Third Person Character` _asbp_third_person_character)
  (`KismetSystemLibrary.K2_SetTimerDelegate` (delegate `Rotate`) 0.01 true true)
  (`self.Mesh_Update` "NewEnumerator0"))

(event `Rotate`
  (bind _root (`self.root`))
  (bind (_relativerotation_roll _relativerotation_pitch _relativerotation_yaw) (`KismetMathLibrary.BreakRotator` (`SceneComponent.RelativeRotation` _root)))
  ;[1 0.587 0 0.5] BeginPlay Setup
  (`SceneComponent.K2_SetRelativeRotation` _root (`KismetMathLibrary.MakeRotator` _relativerotation_roll _relativerotation_pitch (+ _relativerotation_yaw 3.0)) false false))

(event `self.ReceiveActorBeginOverlap`
  (params (OtherActor :type "Actor Object Reference"))
  (if (`self.ActorHasTag` OtherActor "Collision")
    (`KismetArrayLibrary.Array_Add` (`self.Other Actors`) OtherActor)
    (`self.Collision_Update` :!label _label)))

(event `self.ReceiveActorEndOverlap`
  (params (OtherActor :type "Actor Object Reference"))
  (`KismetArrayLibrary.Array_RemoveItem` (`self.Other Actors`) OtherActor)
  (goto _label))

(event `Collision_Update`
  (bind _as_bp_third_person_character (`self.As BP Third Person Character`))
  (bind _trappreviewmesh (`self.TrapPreviewMesh`))
  (bind _returnvalue (> (`KismetArrayLibrary.Array_Length` (`self.Other Actors`)) 0))
  ; Comment
  (set `/Game/Blueprints/BP_ThirdPersonCharacter.CanPlaceTraps` (not _returnvalue) _as_bp_third_person_character)
  (set `/Game/Blueprints/BP_ThirdPersonCharacter.PreviewIsOverlapping` _returnvalue _as_bp_third_person_character)
  (if _returnvalue
    (`PrimitiveComponent.SetMaterial` _trappreviewmesh 0 "/Game/Environment/Traps/TrapsPreviewRed.TrapsPreviewRed")
    (`PrimitiveComponent.SetMaterial` (`self.Cube`) 0 "/Game/Environment/Traps/TrapsPreviewRed.TrapsPreviewRed")
    (else
      (`PrimitiveComponent.SetMaterial` _trappreviewmesh 0 "/Game/Environment/Traps/TrapsPreviewMaterialGreen.TrapsPreviewMaterialGreen")
      (`PrimitiveComponent.SetMaterial` (`self.Cube`) 0 "/Game/Environment/Traps/TrapsPreviewMaterialGreen.TrapsPreviewMaterialGreen"))))

(fn `UserConstructionScript`)